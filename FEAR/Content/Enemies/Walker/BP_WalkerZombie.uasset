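; BP_WalkerZombie is a walker zombie enemy that loses health when shot and dies at zero.
; Health starts at MaxHealth on BeginPlay, and capsule hits from first-person projectiles apply fixed damage to itself through ApplyDamage.
; AnyDamage subtracts and prints health, then on death plays a custom animation, destroys the capsule and removes the actor after a delay.
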(event OnComponentHit(CapsuleComponent)
  (params (HitComponent :type Primitive%20Component%20Object%20Reference) (OtherActor :type Actor%20Object%20Reference) (OtherComp :type Primitive%20Component%20Object%20Reference) (NormalImpulse :type Vector :default "0, 0, 0") (Hit :type Hit%20Result%20Structure%20%28by%20ref%29))
  ;[1 1 1] Zombie takes damage when shot
  (bind _asbp_first_person_projectile (Utilities|Casting|CastToBP_FirstPersonProjectile OtherActor))
  (Game|Damage|ApplyDamage self 1e+01 0 _asbp_first_person_projectile))

(event EventBeginPlay
  (CallFunction|BaseHealth))

(event Collision|EventActorBeginOverlap
  (params (OtherActor :type Actor%20Object%20Reference)))

(event EventTick
  (params (DeltaSeconds :type Float%20%28single-precision%29)))

(event Game|Damage|EventAnyDamage
  (params (Damage :type Float%20%28single-precision%29) (DamageType :type Damage%20Type%20Object%20Reference) (InstigatedBy :type Controller%20Object%20Reference) (DamageCauser :type Actor%20Object%20Reference))
  ;[1 1 1] Zombie takes damage when shot
  (bind _output_get (Variables|Default|SetHealth (- (Variables|Default|GetHealth) Damage)))
  (Development|PrintString (Utilities|String|ToString(Float) _output_get))
  (if (<= (Variables|Default|GetHealth) 0.0)
    (bind _output_get_2 (Variables|Default|SetIsDead true))
    (if _output_get_2
      (Utilities|FlowControl|Sequence
        (:then_0
          (Development|PrintString "Walker Zombie Died")
          (Components|Animation|PlayAnimation (Variables|Character|GetMesh) "/Game/Enemies/Walker/Custom_Death.Custom_Death" false)
          (Utilities|FlowControl|Delay 5.0)
          (Actor|DestroyActor))
        (:then_1
          (Components|DestroyComponent (Variables|Collision|GetCapsuleComponent)))))))

(fn ConstructionScript)

(fn BaseHealth
  (Variables|Default|SetHealth (Variables|Default|GetMaxHealth)))