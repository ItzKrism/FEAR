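; Crawler zombie enemy that hears the player, attacks in melee and dies from damage, reusing Walker-named montage and log text.
; Tick updates the health bar widget and turns it toward the camera.
; Hearing the player sets HasHeardPlayer on the AI blackboard, while AttackPlayer sphere-traces ahead to apply damage with a montage.
; AnyDamage reduces Health and, at zero, removes the capsule, hides the bar, plays death effects and destroys the actor after a delay.
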(event OnHearNoise(PawnSensing)
  (params (Instigator :type Pawn%20Object%20Reference) (Location :type Vector%20%28by%20ref%29 :default "0, 0, 0") (Volume :type Float%20%28single-precision%29))
  ;[0 0 0] Player Made Noise
  (Utilities|Casting|CastToBP_FirstPersonCharacter Instigator)
  (AI|Components|Blackboard|SetValueasBool (AI|GetBlackboard (AI|GetAIController self)) (Utilities|Name|MakeLiteralName "HasHeardPlayer") true))

(event Custom|Attack%20Player
  (bind _returnvalue (Transformation|GetActorLocation))
  ;[0 0 0] Zombie Attack Player
  (bind (_outhit _returnvalue_2) (Collision|SphereTraceForObjects _returnvalue (+ _returnvalue (* (Math|Vector|GetForwardVector (Transformation|GetActorRotation)) 2e+01)) 1.2e+02 (Utilities|Array|MakeArray "ObjectTypeQuery3") false 0 "None" true "(R=1.000000,G=0.000000,B=0.000000,A=1.000000)" "(R=0.000000,G=1.000000,B=0.000000,A=1.000000)" 1.0))
  (if _returnvalue_2
    (Utilities|Casting|CastToBP_FirstPersonCharacter (.HitActor (Collision|BreakHitResult _outhit)))
    (Components|Activation|Deactivate (Variables|Character|GetCharacterMovement))
    (Animation|PlayAnimMontage "/Game/Enemies/Walker/WalkerAnimations/WalkerAnimations/AM_WalkerAttack.AM_WalkerAttack" 1.0 "None")
    (bind _asbp_first_person_character (Utilities|Casting|CastToBP_FirstPersonCharacter (Game|GetPlayerCharacter 0)))
    (Game|Damage|ApplyDamage _asbp_first_person_character 1e+01 0 self)
    (Audio|PlaySoundatLocation 0 (Transformation|GetActorLocation) "0, 0, 0" 1.0 1.0 0.0 0 0 0 0)
    (Components|Activation|Activate (Variables|Character|GetCharacterMovement) false)))

(event EventBeginPlay
  (CallFunction|BaseHealth))

(event Collision|EventActorBeginOverlap
  (params (OtherActor :type Actor%20Object%20Reference)))

(event EventTick
  (params (DeltaSeconds :type Float%20%28single-precision%29))
  (bind _healthbar (Variables|Default|GetHealthBar))
  ;[0 0 0] Zombie Health
  (bind _aswb_enemy_health_bar (Utilities|Casting|CastToWB_EnemyHealthBar (UserInterface|GetWidget (Variables|Default|GetHealthBar))))
  (Progress|SetPercent (Variables|/Game/UI/WB_EnemyHealthBar.WB_EnemyHealthBar_C|GetEnemyHealthBar _aswb_enemy_health_bar) (/ (Variables|Default|GetHealth) (Variables|Default|GetMaxHealth)))
  (Transformation|SetWorldRotation _healthbar (Math|Rotator|FindLookatRotation (Transformation|GetWorldLocation _healthbar) (Transformation|GetWorldLocation (Variables|/Script/Engine.PlayerCameraManager|GetTransformComponent (Game|GetPlayerCameraManager 0)))) false false))

(event Game|Damage|EventAnyDamage
  (params (Damage :type Float%20%28single-precision%29) (DamageType :type Damage%20Type%20Object%20Reference) (InstigatedBy :type Controller%20Object%20Reference) (DamageCauser :type Actor%20Object%20Reference))
  ;[0 0 0] Zombie takes damage when shot
  (CallFunction|DisplayHealth Damage)
  (bind _isbrodead (CallFunction|IsItDead))
  (if _isbrodead
    (Utilities|FlowControl|Sequence
      (:then_0
        (Development|PrintString "Walker Zombie Died")
        (Components|Animation|PlayAnimation (Variables|Character|GetMesh) "/Game/Enemies/Walker/Custom_Death.Custom_Death" false)
        (Utilities|FlowControl|Sequence
          (:then_0
            (Audio|PlaySound2D "/Game/Sounds/ZombieSounds/Zombie-Growling-sound-effect.Zombie-Growling-sound-effect" 1.0 1.0 0.0 0 0))
          (:then_1
            (Utilities|FlowControl|Delay 5.0)
            (Actor|DestroyActor))))
      (:then_1
        (Components|DestroyComponent (Variables|Collision|GetCapsuleComponent))
        (Rendering|SetVisibility (Variables|Default|GetHealthBar) false false)))))

(fn ConstructionScript)

(fn BaseHealth
  (Variables|Default|SetHealth (Variables|Default|GetMaxHealth)))

(fn DisplayHealth
  (params (ZombieHP :type Float%20%28double-precision%29))
  (Variables|Default|SetHealth (- (Variables|Default|GetHealth) ZombieHP)))

(fn IsItDead
  (if (<= (Variables|Default|GetHealth) 0.0)
    (bind _output_get (Variables|Default|SetIsDead true))
    (return _output_get)))