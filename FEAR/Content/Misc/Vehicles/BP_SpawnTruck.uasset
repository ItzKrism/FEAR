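; BP_SpawnTruck is a vehicle Blueprint that flashes a red and blue siren light.
; BeginPlay starts an endless loop that waits MaxTime on a retriggerable delay, then calls SirenFlashing.
; SirenFlashing uses a FlipFlop to alternate which point light gets the bright intensity and which gets the dim one.
; The file contains no spawning or driving logic, and the construction script is empty.
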(event EventBeginPlay
  (Utilities|FlowControl|RetriggerableDelay (Variables|Default|GetMax%20Time) :!label _label)
  (CallFunction|SirenFlashing)
  (goto _label))

(fn ConstructionScript)

(fn SirenFlashing
  (Utilities|FlowControl|FlipFlop
    (:A
      (Rendering|Components|Light|SetIntensity (Variables|Default|GetPointLightRed) (Variables|Default|GetDim%20Intensity))
      (Rendering|Components|Light|SetIntensity (Variables|Default|GetPointLightBlue) (Variables|Default|GetIntensity)))
    (:B
      (Rendering|Components|Light|SetIntensity (Variables|Default|GetPointLightRed) (Variables|Default|GetIntensity))
      (Rendering|Components|Light|SetIntensity (Variables|Default|GetPointLightBlue) (Variables|Default|GetDim%20Intensity)))))