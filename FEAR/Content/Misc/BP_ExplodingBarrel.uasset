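; Exploding barrel actor that blows up and damages the player once its BarrelHit flag is set.
; Tick polls the flag, activates the particle system and explosion collision, then destroys the actor.
; Component activation events play the sound and apply damage if IsInRadius is set.
; Any overlap latches IsInRadius, damage always targets the first-person player, and the walker zombie damage code is unconnected.
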(event OnComponentActivated(ExplosionCollision)
  (params (Component :type Actor%20Component%20Object%20Reference) (bReset :type Boolean))
  (if (Variables|Default|GetIsInRadius)
    (CallFunction|DealDamageExplosive)))

(event OnComponentActivated(ParticleSystem)
  (params (Component :type Actor%20Component%20Object%20Reference) (bReset :type Boolean))
  (Audio|PlaySoundatLocation "/Game/StarterContent/Audio/Explosion01.Explosion01" (Transformation|GetWorldLocation (Variables|Default|GetParticleSystem)) "0, 0, 0" 1.0 1.0 0.0 0 0 0 0))

(event OnComponentBeginOverlap(ExplosionCollision)
  (params (OverlappedComponent :type Primitive%20Component%20Object%20Reference) (OtherActor :type Actor%20Object%20Reference) (OtherComp :type Primitive%20Component%20Object%20Reference) (OtherBodyIndex :type Integer) (bFromSweep :type Boolean) (SweepResult :type Hit%20Result%20Structure%20%28by%20ref%29))
  (if true
    (Variables|Default|SetIsInRadius true)))

(event EventBeginPlay
  (Components|Activation|Deactivate (Variables|Default|GetExplosionCollision)))

(event Collision|EventActorBeginOverlap
  (params (OtherActor :type Actor%20Object%20Reference)))

(event EventTick
  (params (DeltaSeconds :type Float%20%28single-precision%29))
  (if (Variables|Default|GetBarrelHit)
    (Components|Activation|Activate (Variables|Default|GetParticleSystem) false)
    (Components|Activation|Activate (Variables|Default|GetExplosionCollision) false)
    (Actor|DestroyActor)))

(fn ConstructionScript)

(fn DealDamageExplosive
  (Utilities|FlowControl|Sequence
    (:then_0
      (bind _asbp_first_person_character (Utilities|Casting|CastToBP_FirstPersonCharacter (Game|GetPlayerCharacter 0)))
      (Game|Damage|ApplyDamage _asbp_first_person_character 5e+01 0 0))))